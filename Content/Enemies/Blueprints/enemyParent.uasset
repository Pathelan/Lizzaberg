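; Base enemy character that chases the player and is destroyed when its health runs out.
; BeginPlay sets current health and walk speed from the max health and move speed variables, then starts a self-restarting AIMoveTo loop.
; Each move targets the player's location at that moment and restarts shortly after success or failure.
; EnemyDamage only subtracts health, while Tick polls it to destroy the actor.
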(event Custom|Enemy%20Move
  (AI|AIMoveTo self (Transformation|GetActorLocation (Game|GetPlayerCharacter 0)) 0 5.0 false
    (:OnSuccess
      (Utilities|FlowControl|Delay 0.1))
    (:OnFail
      (Utilities|FlowControl|Delay 0.1)))
  (CallFunction|EnemyMove))

(event EventBeginPlay
  (CallFunction|SetVariables)
  (CallFunction|EnemyMove))

(event Collision|EventActorBeginOverlap
  (params (OtherActor :type Actor%20Object%20Reference)))

(event EventTick
  (params (DeltaSeconds :type Float%20%28single-precision%29))
  (if (<= (Variables|Default|GetenemyCurrentHealth) 0.0)
    (Actor|DestroyActor)))

(event EventEnemyDamage
  (params (Damage :type Float%20%28double-precision%29))
  (bind _output_get (Variables|Default|SetenemyCurrentHealth (- (Variables|Default|GetenemyCurrentHealth) Damage)))
  (if (<= _output_get 0.0)
    _))

(fn ConstructionScript)

(fn SetVariables
  (Utilities|FlowControl|Sequence
    (:then_0
      (Variables|Default|SetenemyCurrentHealth (Variables|Default|GetenemyMaxHealth)))
    (:then_1
      (Variables|/Script/Engine.CharacterMovementComponent|SetMaxWalkSpeed (Variables|Character|GetCharacterMovement) (Variables|Default|GetenemyMoveSpeed)))))